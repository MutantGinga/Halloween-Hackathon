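; BP_Ghost is a ghost actor that shows itself only when the player is close and vanishes when photographed.
; BeginPlay assigns the OooOoooO sound to its Sound component.
; Every Tick toggles GhostBody visibility by comparing its distance to the player character's mesh against MinDistance.
; The PhotoTaken event destroys the actor, and leftover debug prints of locations and distance never run.
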(event Custom|PhotoTaken
  (Actor|DestroyActor))

(event EventBeginPlay
  (Audio|Components|Audio|SetSound (Variables|Default|GetSound) "/Game/Audio/OooOoooO.OooOoooO"))

(event Collision|EventActorBeginOverlap
  (params (OtherActor :type Actor%20Object%20Reference)))

(event EventTick
  (params (DeltaSeconds :type Float%20%28single-precision%29))
  (Rendering|SetVisibility (Variables|Default|GetGhostBody) (< (Math|Vector|VectorLength (- (Transformation|GetWorldLocation (Variables|Default|GetGhostBody)) (Transformation|GetWorldLocation (Variables|/Script/Engine.Character|GetMesh (Game|GetPlayerCharacter 0))))) (Variables|Default|GetMinDistance)) false))

(fn ConstructionScript)